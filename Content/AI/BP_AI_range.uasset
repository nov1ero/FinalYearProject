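; BP_AI_range is an AI combat character that reacts to damage and can attack.
; On damage it plays a random hit montage, prints the amount and launches itself along the player character's forward vector.
; Attack plays a sword slash montage, GetAttackRange returns zero, and Ragdolll switches off mesh physics after a short delay.
; Learning Agents manager registration is present but disconnected from BeginPlay.
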(event Custom|Ragdolll
  (Utilities|FlowControl|Delay 0.2)
  (Physics|SetSimulatePhysics (Variables|Character|GetMesh) false))

(event EventBeginPlay
  ;[1 1 1] Register agents with manager
)

(event Game|Damage|EventAnyDamage
  (params (Damage :type Float%20%28single-precision%29) (DamageType :type Damage%20Type%20Object%20Reference) (InstigatedBy :type Controller%20Object%20Reference) (DamageCauser :type Actor%20Object%20Reference))
  ;[0.01764 0.01764 0.01764] Recieve Damage
  (Animation|PlayAnimMontage (Utilities|Array|Get(acopy) (Variables|Default|GetHitAnims) (Math|Random|RandomIntegerinRange 0 (- (Utilities|Array|Length (Variables|Default|GetHitAnims)) 1))) 1.0 "None")
  (Development|PrintString (Utilities|String|ToString(Float) Damage))
  (bind _asbp_top_down_character (Utilities|Casting|CastToBP_TopDownCharacter (Game|GetPlayerCharacter 0)))
  (Character|LaunchCharacter (* (Math|Vector|GetForwardVector (Transformation|GetActorRotation _asbp_top_down_character)) 7e+02) false false))

(fn ConstructionScript)

(fn GetAttackRange
  (return 0.0))

(fn Attack
  (bind _returnvalue (Animation|PlayAnimMontage "/Game/Characters/Player/Animations/Attack/NormalAttack/Anim_SwordV2_Slash1_Montage.Anim_SwordV2_Slash1_Montage" 1.0 "None"))
  (return _returnvalue))