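; Melee AI character that registers itself as an agent with the level's LearningAgentsManager on BeginPlay.
; It spawns a sword onto its hand socket, plays a slash montage to attack and sets walk speed by movement state.
; Damage plays a random hit montage and lowers StatsComponent health, then either knocks it along the player's facing or simulates mesh physics on death.
; Attack range, patrol route and health-decrease functions are unimplemented stubs.
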(event Custom|Ragdolll
  (Utilities|FlowControl|Delay 0.2)
  (Physics|SetSimulatePhysics (Variables|Character|GetMesh) false))

(event Custom|WieldSword
  (bind _returnvalue (Game|SpawnActorfromClass "/Game/Characters/Doll/weopon/BP_Sword.BP_Sword_C" (Transformation|GetActorTransform) "Undefined" "MultiplyWithRoot" 0 0))
  (Transformation|AttachComponentToComponent _returnvalue (Variables|Character|GetMesh) "Weapon_R" "SnapToTarget" "SnapToTarget" "SnapToTarget" true)
  (Variables|Default|SetIsWieldingSword true))

(event EventBeginPlay
  ;[1 1 1] Register agents with manager
  (bind _returnvalue (Actor|GetActorOfClass "/Script/LearningAgents.LearningAgentsManager"))
  (Utilities|IsValid _returnvalue
    (:Is%20Valid
      (bind _returnvalue_2 (Class|LearningAgentsManager|AddAgent _returnvalue self))
      (Variables|Default|SetAgent%20Id _returnvalue_2))
    (:Is%20Not%20Valid
      (Development|PrintString "Could not find Learning Agents manager. Did we forget to add one to the scene?"))))

(event Game|Damage|EventAnyDamage
  (params (Damage :type Float%20%28single-precision%29) (DamageType :type Damage%20Type%20Object%20Reference) (InstigatedBy :type Controller%20Object%20Reference) (DamageCauser :type Actor%20Object%20Reference))
  (bind _statscomponent (Variables|Default|GetStatsComponent))
  ;[0.01764 0.01764 0.01764] Recieve Damage
  (Animation|PlayAnimMontage (Utilities|Array|Get(acopy) (Variables|Default|GetHitAnims) (Math|Random|RandomIntegerinRange 0 (- (Utilities|Array|Length (Variables|Default|GetHitAnims)) 1))) 1.0 "None")
  (bind _output_get (Variables|/Game/TopDown/Blueprints/StatsComponent.StatsComponent_C|SetCurrentHealth _statscomponent (- (Variables|/Game/TopDown/Blueprints/StatsComponent.StatsComponent_C|GetCurrentHealth _statscomponent) Damage)))
  (if (<= _output_get 0.0)
    (Input|DisableInput 0)
    (Physics|SetSimulatePhysics (Variables|Character|GetMesh) true)
    (else
      (bind _asbp_top_down_character (Utilities|Casting|CastToBP_TopDownCharacter (Game|GetPlayerCharacter 0)))
      (Character|LaunchCharacter (* (Math|Vector|GetForwardVector (Transformation|GetActorRotation _asbp_top_down_character)) 7e+02) false false))))

(fn ConstructionScript)

(fn GetAttackRange
  (return 0.0))

(fn Decreasehealth)

(fn Attack
  (bind _returnvalue (Animation|PlayAnimMontage "/Game/Characters/Player/Animations/Attack/NormalAttack/Anim_SwordV2_Slash1_Montage.Anim_SwordV2_Slash1_Montage" 1.0 "None"))
  (return _returnvalue))

(fn GetPatrolRout
  (return false))

(fn SetMovementSpeed
  (params (Speed :type Enum_AI_MovementSpeed%20Enum :default "NewEnumerator0"))
  (Variables|/Script/Engine.CharacterMovementComponent|SetMaxWalkSpeed (Variables|Character|GetCharacterMovement) (Utilities|Select :Index Speed :NewEnumerator0 0.0 :NewEnumerator1 2.5e+02 :NewEnumerator2 4e+02 :NewEnumerator3 0.0))
  (return 0.0))