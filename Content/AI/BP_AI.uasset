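; AI character Blueprint that reacts to any damage with a random hit animation montage from the HitAnims array and prints the damage amount.
; A separate Ragdolll event waits briefly, then turns physics simulation off on the mesh; nothing in the graph enables it or calls the event.
; The graph tracks no health or death, and the construction script is empty.
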(event Custom|Ragdolll
  (Utilities|FlowControl|Delay 0.2)
  (Physics|SetSimulatePhysics (Variables|Character|GetMesh) false))

(event Game|Damage|EventAnyDamage
  (params (Damage :type Float%20%28single-precision%29) (DamageType :type Damage%20Type%20Object%20Reference) (InstigatedBy :type Controller%20Object%20Reference) (DamageCauser :type Actor%20Object%20Reference))
  (Animation|PlayAnimMontage (Utilities|Array|Get(acopy) (Variables|Default|GetHitAnims) (Math|Random|RandomIntegerinRange 0 (- (Utilities|Array|Length (Variables|Default|GetHitAnims)) 1))) 1.0 "None")
  (Development|PrintString (Utilities|String|ToString(Float) Damage)))

(fn ConstructionScript)