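; Learning Agents interactor for BP_AI_melee fighters that defines what each agent observes about an enemy.
; Setup registers planar position, direction and velocity observations for the enemy.
; Each update converts the stored enemy values relative to the agent's location and rotation, with velocity relative to its movement heading.
; Action setup and retrieval are disabled stubs, and the enemy values are not assigned here.
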(event EventSetupObservations
  (Utilities|FlowControl|Sequence
    (:then_0
      (bind _returnvalue (Class|PlanarPositionObservation|AddPlanarPositionObservation 0 "EnemyPosition" 5e+02 "1.000000,0.000000,0.000000" "0.000000,1.000000,0.000000"))
      (Variables|Default|SetEnemyPositionObservation _returnvalue)
      (bind _returnvalue_2 (Class|PlanarDirectionObservation|AddPlanarDirectionObservation 0 "EnemyDirectionObservation" 1.0 "1.000000,0.000000,0.000000" "0.000000,1.000000,0.000000"))
      (Variables|Default|SetEnemyDirectionObservation _returnvalue_2)
      (bind _returnvalue_3 (Class|PlanarVelocityObservation|AddPlanarVelocityObservation 0 "EnemyVelocity" 2e+02 "1.000000,0.000000,0.000000" "0.000000,1.000000,0.000000"))
      (Variables|Default|SetEnemyVelocityObservation _returnvalue_3))))

(event EventSetObservations
  (params (AgentIds :type Array%20of%20Integers))
  (for _array_element AgentIds
    (Utilities|FlowControl|Sequence
      (:then_0
        (Class|PlanarPositionObservation|SetPlanarPositionObservation (Variables|Default|GetEnemyPositionObservation) _array_element (Variables|Default|GetEnemyPosition) (Transformation|GetActorLocation (Class|LearningAgentsManagerComponent|GetAgent _array_element "/Game/AI/BP_AI_melee.BP_AI_melee_C")) (Transformation|GetActorRotation (Class|LearningAgentsManagerComponent|GetAgent _array_element "/Game/AI/BP_AI_melee.BP_AI_melee_C"))))
      (:then_1
        (Class|PlanarDirectionObservation|SetPlanarDirectionObservation (Variables|Default|GetEnemyDirectionObservation) _array_element (Variables|Default|GetEnemyDirection) (Transformation|GetActorRotation (Class|LearningAgentsManagerComponent|GetAgent _array_element "/Game/AI/BP_AI_melee.BP_AI_melee_C"))))
      (:then_2
        (Class|PlanarVelocityObservation|SetPlanarVelocityObservation (Variables|Default|GetEnemyVelocityObservation) _array_element (Variables|Default|GetEnemyVelocity) (Math|Conversions|RotationFromXVector (Transformation|GetVelocity (Class|LearningAgentsManagerComponent|GetAgent _array_element "/Game/AI/BP_AI_melee.BP_AI_melee_C"))))))))

(event EventSetupActions)

(event EventGetActions
  (params (AgentIds :type Array%20of%20Integers)))