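; Learning Agents manager for recording BP_AI_range fight behavior as training data, apparently unfinished.
; Tick loops over all agents, calls controller EncodeActions, then adds the experience to the fight recorder.
; The per-agent RecordPlayerForTick only fetches the agent.
; Agent spawning, recorder and controller setup, timed recording sessions, observation encoding and interactor setup are all disconnected, so BeginPlay does nothing.
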(event EventBeginPlay)

(event Collision|EventActorBeginOverlap
  (params (OtherActor :type Actor%20Object%20Reference)))

(event EventTick
  (params (DeltaSeconds :type Float%20%28single-precision%29))
  (bind _outagentids (Class|LearningAgentsManager|GetAllAgents "/Game/AI/BP_AI_range.BP_AI_range_C"))
  (for (_ _array_index) _outagentids
    (CallFunction|RecordPlayerforTick _array_index))
  (Class|LearningAgentsController|EncodeActions (Variables|Default|GetBP_LAController))
  (Class|LearningAgentsRecorder|AddExperience (Variables|Default|GetBP_FightRecorder)))

(fn ConstructionScript)

(fn SpawnAgent)

(fn SpawnEnemy
  (params (Id :type Integer))
  (bind _output_get (Variables|Default|SetY%20shift (* "" (Variables|Default|GetId))))
  (bind _returnvalue (Game|SpawnActorfromClass "/Game/AI/BP_AI_range.BP_AI_range_C" (Math|Transform|MakeTransform (+ _output_get (.location (Transformation|GetActorTransform))) "0, 0, 0" "1.000000,1.000000,1.000000") "Undefined" "MultiplyWithRoot" 0 0))
  (bind _returnvalue_2 (Class|LearningAgentsManager|AddAgent _returnvalue))
  (Variables|Default|SetId _returnvalue_2)
  (Variables|Default|SetTarget _returnvalue))

(fn RecordPlayerforTick
  (params (Agent%20Id :type Integer))
  (Variables|Default|SetToRecord (Class|LearningAgentsManager|GetAgent Agent%20Id "/Game/AI/BP_AI_range.BP_AI_range_C")))